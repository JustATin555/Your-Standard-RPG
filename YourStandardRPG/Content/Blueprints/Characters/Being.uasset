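; Being is a character Blueprint that manages Health and Mana.
; AnyDamage switches on the damage type's display name: the healing type subtracts Damage from Health with clamping to MaxHealth, while other types subtract it unclamped and print the type name.
; Tick regenerates Mana by ManaRegen over time up to MaxMana, and CheckForMana reports whether a given cost is affordable.
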(event EventTick
  (params (DeltaSeconds :type Float%20%28single-precision%29))
  (Utilities|FlowControl|Sequence
    (:then_0
      ;[1 1 1] Mana Regen
      (Variables|Default|SetMana (Math|Float|Clamp(Float) (+ (Variables|Default|GetMana) (* (Variables|Default|GetMana%20Regen) DeltaSeconds)) 0.0 (Variables|Default|GetMax%20Mana))))))

(event Game|Damage|EventAnyDamage
  (params (Damage :type Float%20%28single-precision%29) (DamageType :type Damage%20Type%20Object%20Reference) (InstigatedBy :type Controller%20Object%20Reference) (DamageCauser :type Actor%20Object%20Reference))
  (bind _returnvalue (Utilities|GetDisplayName DamageType))
  ;[1 1 1] Switch for Damage Types
  (switch string _returnvalue
    (:Default
      (Variables|Default|SetHealth (- (Variables|Default|GetHealth) Damage))
      (Development|PrintString _returnvalue))
    (:Default__Healing_C
      ;[1 1 1] Healing
      (Variables|Default|SetHealth (Math|Float|Clamp(Float) (- (Variables|Default|GetHealth) Damage) 0.0 (Variables|Default|GetMax%20Health))))))

(fn ConstructionScript)

(fn CheckforMana
  (params (Mana%20Cost :type Float%20%28single-precision%29))
  (return (<= Mana%20Cost (Variables|Default|GetMana))))